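; BP_RigelPawn is a pawn Blueprint that reads model metadata from components picked in the scene.
; On BeginPlay it binds a handler to OnPickEvent, which reads the picked component's first property table and primitive metadata.
; The handler loops over property names and attribute indices and looks up an empty property key, but nothing acts on the results, so it appears unfinished.
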(event `self.ReceiveBeginPlay`
  (add `self.OnPickEvent` (delegate `OnPickEvent_Event`)))

(event `OnPickEvent_Event` :!signature `self.OnPickEvent`
  (params (PickActor :type "Actor Object Reference") (PickComponent :type "PrimitiveComponent Object Reference"))
  (bind _returnvalue (`CesiumModelMetadataBlueprintLibrary.GetPropertyTable` (`CesiumModelMetadataBlueprintLibrary.GetModelMetadata` PickComponent)))
  (for _ (`CesiumPropertyTableBlueprintLibrary.GetPropertyNames` _returnvalue)
    _)
  (for _ (`CesiumPrimitiveMetadataBlueprintLibrary.GetPropertyAttributeIndices` (`CesiumPrimitiveMetadataBlueprintLibrary.GetPrimitiveMetadata` PickComponent))
    _)
  (if (`.ReturnValue` (`BlueprintMapLibrary.Map_Find` (`CesiumPropertyTableBlueprintLibrary.GetProperties` _returnvalue)))
    _))

(fn `UserConstructionScript`)