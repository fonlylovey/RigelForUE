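; Rigel interface Blueprint that switches the level's lighting between day and night.
; ChangeLight finds the LightPost and NightPost post-process volumes through RigelLevel and enables one while disabling the other.
; SetTimeOfDay is empty; disconnected nodes hold Ultra Dynamic Sky time parsing from JSON, day/night forwarding to BP_Terrain, and paired sky and fog presets.
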(event `self.SetTimeOfDay`
  (params (DataObj :type "JsonLibraryObject Structure (by ref)")))

(event `ChangeLight`
  (params (IsLight :type Boolean))
  (if IsLight
    (bind _returnvalue (`RigelLevelEditor.RigelLevel`))
    (bind _returnvalue_2 (`RigelLevelEditor.FindActor` _returnvalue "LightPost"))
    (bind `_as后期处理体积` (cast `PostProcessVolume` _returnvalue_2))
    (set `PostProcessVolume.bEnabled` true `_as后期处理体积`)
    (bind _returnvalue_3 (`RigelLevelEditor.FindActor` _returnvalue "NightPost"))
    (bind `_as后期处理体积_2` (cast `PostProcessVolume` _returnvalue_3))
    (set `PostProcessVolume.bEnabled` false `_as后期处理体积_2`)
    (else
      (bind _returnvalue_4 (`RigelLevelEditor.RigelLevel`))
      (bind _returnvalue_5 (`RigelLevelEditor.FindActor` _returnvalue_4 "LightPost"))
      (bind `_as后期处理体积_3` (cast `PostProcessVolume` _returnvalue_5))
      (set `PostProcessVolume.bEnabled` false `_as后期处理体积_3`)
      (bind _returnvalue_6 (`RigelLevelEditor.FindActor` _returnvalue_4 "NightPost"))
      (bind `_as后期处理体积_4` (cast `PostProcessVolume` _returnvalue_6))
      (set `PostProcessVolume.bEnabled` true `_as后期处理体积_4`))))