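; Rigel level script for a Cesium georeferenced map app, serving as the bridge between a web widget UI and the 3D scene.
; At BeginPlay it registers JSON-driven API handlers for POIs, map layers, material parameters, people paths and video playback.
; POIs spawn by style or device type at geographic coordinates, either directly or through a quadtree updated on map level changes.
; It also toggles building VFX by zoom level and highlights picked project components.
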(event `self.ReceiveBeginPlay`
  (bind _returnvalue (`self.RigelLevel`))
  (if (== (`RigelLevelEditor.StreamMode` _returnvalue) 0)
    (bind _returnvalue_2 (`|CreateWidget` "/Rigel/Blueprints/UMG/BP_WebWidget.BP_WebWidget_C" (`GameplayStatics.GetPlayerController` 0)))
    (`UserWidget.AddToViewport` _returnvalue_2 0)
    (bind _asrigel_pawn (cast `RigelPawn` (`GameplayStatics.GetPlayerPawn` 0)))
    (set `self.RigelPawn` _asrigel_pawn)
    (`|ExecutionSequence`
      (:`then_0`
        (add `RigelPawn.OnPickEvent` (`self.RigelPawn`) (`|CreateDelegate` :!event `OnClickedEvent`)))
      (:`then_2`
        (add `RigelPawn.OnMapLevelChange` (`self.RigelPawn`) (`|CreateDelegate` :!event `OnMapLevelChange_Event`))
        (bind _returnvalue_3 (`RigelAPISubsystem.RigelAPISubsystem`))
        (`RigelAPISubsystem.Register` _returnvalue_3 "ClearQuadtreeScene" (`|CreateDelegate` :!event `ClearQuadtreeScene`))
        (`RigelAPISubsystem.Register` _returnvalue_3 "PlayerMedia" (`|CreateDelegate` :!event `PlayerMedia`))
        (`RigelAPISubsystem.Register` _returnvalue_3 "QuitGame" (delegate `QuitGame`)))
      (:`then_3`
        (bind _returnvalue_4 (`RigelAPISubsystem.RigelAPISubsystem`))
        (`RigelAPISubsystem.Register` _returnvalue_4 "SetRigelScalarParameter" (`|CreateDelegate` :!event `SetRigelScalarParameter`))
        (`RigelAPISubsystem.Register` _returnvalue_4 "ChangeMapSource" (`|CreateDelegate` :!event `ChangeMapSource`)))
      (:`then_4`
        (bind _returnvalue_5 (`RigelAPISubsystem.RigelAPISubsystem`))
        (`RigelAPISubsystem.Register` _returnvalue_5 "SetPipeVectorLayer" (`|CreateDelegate` :!event `Set Pipe Vector Layer`))
        (`RigelAPISubsystem.Register` _returnvalue_5 "SetPeoplePathPoints" (`|CreateDelegate` :!event `SetPeoplePathPoints`)))
      (:`then_5`
        (bind _returnvalue_6 (`RigelAPISubsystem.RigelAPISubsystem`))
        (`RigelAPISubsystem.Register` _returnvalue_6 "CreatePOI" (delegate `CreatePOI`))
        (`RigelAPISubsystem.Register` _returnvalue_6 "SetPeopleAnimationPath" (`|CreateDelegate` :!event `SetPeopleAnimationPath`))
        (`RigelAPISubsystem.Register` _returnvalue_6 "CreatePOIByDataList" (`|CreateDelegate` :!event `CreatePOIByDataList`)))
      (:`then_6`
        (bind _returnvalue_7 (`RigelAPISubsystem.RigelAPISubsystem`))
        (`RigelAPISubsystem.Register` _returnvalue_7 "SetServerVisible" (`|CreateDelegate` :!event `SetServerVisible`))))))

(event `SetRigelScalarParameter`
  (params (Value :type "JsonLibraryObject Structure (by ref)"))
  (bind _returnvalue (`JsonLibraryHelpers.JsonObject_GetFloat` Value "Value"))
  (bind _returnvalue_2 (`KismetStringLibrary.Conv_StringToName` (`JsonLibraryHelpers.JsonObject_GetString` Value "Parameter")))
  ;[1 1 1] Rigel API
  (if (== (`JsonLibraryHelpers.JsonObject_GetString` Value "MPCName") "Project")
    (`KismetMaterialLibrary.SetScalarParameterValue` "/Game/Base/Materials/MPC_Project.MPC_Project" _returnvalue_2 _returnvalue)
    (else
      (`KismetMaterialLibrary.SetScalarParameterValue` "/Rigel/Materials/MPC_RigelParaCollection.MPC_RigelParaCollection" _returnvalue_2 _returnvalue))))

(event `SetRigelVectorParameter`
  (params (Value :type "JsonLibraryObject Structure (by ref)"))
  ;[1 1 1] Rigel API
  (`KismetMaterialLibrary.SetScalarParameterValue` "/Rigel/Materials/MPC_RigelParaCollection.MPC_RigelParaCollection" "EmissiveLight"))

(event `QuitGame`
  (params (Value :type "JsonLibraryObject Structure (by ref)"))
  (`KismetSystemLibrary.QuitGame` null "Quit"))

(event `SetPeopleAnimationPath`
  (params (jsonData :type "JsonLibraryObject Structure"))
  ;[1 1 1] Rigel API
  (bind _returnvalue (`self.GetRuntimeActor` (`JsonLibraryHelpers.JsonObject_GetString` jsonData "ActorID")))
  (bind _returnvalue_2 (`self.GetActor` (`JsonLibraryHelpers.JsonObject_GetString` jsonData "PathID")))
  (if (and (`KismetSystemLibrary.IsValid` _returnvalue_2) (`KismetSystemLibrary.IsValid` _returnvalue))
    (bind _asbp_poi_people_status (cast `/Game/SHContent/POI/BP_POI_PeopleStatus` _returnvalue))
    (bind _asspline_path_mesh (cast `SplinePathMesh` _returnvalue_2))
    (bind _animationpath (`/Game/SHContent/POI/BP_POI_PeopleStatus.AnimationPath` _asbp_poi_people_status))
    (set `AnimationPathComponent.SplineActor` _asspline_path_mesh _animationpath)
    (`AnimationPathComponent.PlayAnimationPath` _animationpath)
    (bind _returnvalue_3 (`self.GetActor` "BP_SplineMeshAnalysis6"))
    (`/Engine/EditorBlueprintResources/StandardMacros.IsValid` _returnvalue_3
      (:`Is Valid`
        (`self.SetActorHiddenInGame` _returnvalue_3 false)))))

(event `ChangeMapSource`
  (params (JsonData :type "JsonLibraryObject Structure"))
  ;[1 1 1] Rigel API
  (switch `string` (`JsonLibraryHelpers.JsonObject_GetString` JsonData "MapType")
    (:`ImageMap`
      (`ActorComponent.SetActive` (`self.FindComponentByTag` (`self.World`) "/Script/CesiumRuntime.CesiumWebMapServiceRasterOverlay" "VectorMap") false false)
      (`ActorComponent.SetActive` (`self.FindComponentByTag` (`self.World`) "/Script/CesiumRuntime.CesiumTileMapServiceRasterOverlay" "ImageMap") true false)
      (`ActorComponent.SetActive` (`self.FindComponentByTag` (`self.World`) "/Script/CesiumRuntime.CesiumWebMapServiceRasterOverlay" "VectorPipe") false false))
    (:`VectorMap`
      (`ActorComponent.SetActive` (`self.FindComponentByTag` (`self.World`) "/Script/CesiumRuntime.CesiumWebMapServiceRasterOverlay" "VectorMap") true false)
      (`ActorComponent.SetActive` (`self.FindComponentByTag` (`self.World`) "/Script/CesiumRuntime.CesiumTileMapServiceRasterOverlay" "ImageMap") false false)
      (`ActorComponent.SetActive` (`self.FindComponentByTag` (`self.World`) "/Script/CesiumRuntime.CesiumWebMapServiceRasterOverlay" "VectorPipe") true false)))
  (`Cesium3DTileset.RefreshTileset` (`self.World`)))

(event `CreatePOI`
  (params (Value :type "JsonLibraryObject Structure (by ref)"))
  (`self.CreatePOIActor` Value))

(event `HandleQXSY`
  (params (isHidden :type Boolean)))

(event `OnMapLevelChange_Event`
  (params (OldLevel :type Integer) (Level :type Integer))
  (`|ExecutionSequence`
    (:`then_0`
      (`QuadtreeSceneComponent.Update` (`self.QuadtreeScene`) Level))
    (:`then_1`
      (if (>= Level 11)
        _))
    (:`then_2`
      (if (>= Level 12)
        _))
    (:`then_3`
      (if (>= Level 11)
        _))
    (:`then_5`
      (if (> Level 13)
        (bind _returnvalue (`self.FindActor` "BP_VFX_BaiMo"))
        (if (`SceneComponent.bHiddenInGame` (`Actor.RootComponent` _returnvalue))
          _
          (elif (`Actor.bHidden` _returnvalue)
            (bind _asbp_vfx_bai_mo (cast `/Game/VFX/DiKuai_VFX/Models/BP_VFX_BaiMo` _returnvalue))
            (`self.SetActorHiddenInGame` _asbp_vfx_bai_mo false)
            (bind _returnvalue_2 (`JsonLibraryHelpers.ParseObject` "{\"Play\":true}"))
            (`/Game/VFX/DiKuai_VFX/Models/BP_VFX_BaiMo.SetStartBuilding` _asbp_vfx_bai_mo _returnvalue_2)))
        (else
          (bind _returnvalue_3 (`self.FindActor` "BP_VFX_BaiMo"))
          (if (`SceneComponent.bHiddenInGame` (`Actor.RootComponent` _returnvalue_3))
            _
            (elif (not (`Actor.bHidden` _returnvalue_3))
              (bind _asbp_vfx_bai_mo_2 (cast `/Game/VFX/DiKuai_VFX/Models/BP_VFX_BaiMo` _returnvalue_3))
              (bind _returnvalue_4 (`JsonLibraryHelpers.ParseObject` "{\"Play\":false}"))
              (`/Game/VFX/DiKuai_VFX/Models/BP_VFX_BaiMo.SetStartBuilding` _asbp_vfx_bai_mo_2 _returnvalue_4)
              (`KismetSystemLibrary.Delay` 3.0)
              (`self.SetActorHiddenInGame` _asbp_vfx_bai_mo_2 true))))))))

(event `self.QuadtreeScene.OnSpawnPOI`
  (params (POIData :type "POIData Structure (by ref)"))
  (`self.CreatePOIByData` POIData))

(event `self.QuadtreeScene.OnDeletePOI`
  (params (POIData :type "POIData Structure (by ref)"))
  (`self.DeletePOIByData` POIData))

(fn `ClearQuadtreeScene`
  (params (JsonData :type "JsonLibraryObject Structure"))
  (`QuadtreeSceneComponent.ClearAllNode` (`self.QuadtreeScene`)))

(fn `CreateDevice`
  (params (JsonData :type "JsonLibraryObject Structure"))
  (returns (POIActor :type "/Game/SHContent/Blueprint/BP_POIBase Object Reference"))
  (locals (thePOI :type "/Game/SHContent/Blueprint/BP_POIBase Object Reference"))
  (bind _returnvalue (`JsonLibraryHelpers.JsonObject_GetObject` JsonData "JsonValue"))
  (bind _enginecoordinates (`GeoReferencingSystem.GeographicToEngine` (`GeoReferencingSystem.GetGeoReferencingSystem`) (make `GeographicCoordinates` (`JsonLibraryHelpers.JsonObject_GetFloat` JsonData "X") (`JsonLibraryHelpers.JsonObject_GetFloat` JsonData "Y") -204.0)))
  (switch `int` (`JsonLibraryHelpers.JsonObject_GetInteger` _returnvalue "deviceType")
    (:`1`
      (bind _returnvalue_2 (`|SpawnActorFromClass` "/Game/SHContent/POI/BP_POI_Device_LLJ.BP_POI_Device_LLJ_C" (`KismetMathLibrary.MakeTransform` _enginecoordinates) "AlwaysSpawn" "MultiplyWithRoot" null null))
      (set `local.thePOI` _returnvalue_2))
    (:`2`
      (bind _returnvalue_3 (`|SpawnActorFromClass` "/Game/SHContent/POI/BP_POI_Device_YWJ.BP_POI_Device_YWJ_C" (`KismetMathLibrary.MakeTransform` _enginecoordinates) "AlwaysSpawn" "MultiplyWithRoot" null null))
      (set `local.thePOI` _returnvalue_3))
    (:`3`
      (bind _returnvalue_4 (`|SpawnActorFromClass` "/Game/SHContent/POI/BP_POI_Device_ZNBZ.BP_POI_Device_ZNBZ_C" (`KismetMathLibrary.MakeTransform` _enginecoordinates) "AlwaysSpawn" "MultiplyWithRoot" null null))
      (set `local.thePOI` _returnvalue_4))
    (:`4`
      (bind _returnvalue_5 (`|SpawnActorFromClass` "/Game/SHContent/POI/BP_POI_Device_SZJCY.BP_POI_Device_SZJCY_C" (`KismetMathLibrary.MakeTransform` _enginecoordinates) "AlwaysSpawn" "MultiplyWithRoot" null null))
      (set `local.thePOI` _returnvalue_5))
    (:`5`
      (bind _returnvalue_6 (`|SpawnActorFromClass` "/Game/SHContent/POI/BP_POI_Device_QTJC.BP_POI_Device_QTJC_C" (`KismetMathLibrary.MakeTransform` _enginecoordinates) "AlwaysSpawn" "MultiplyWithRoot" null null))
      (set `local.thePOI` _returnvalue_6))
    (:`6`
      (bind _returnvalue_7 (`|SpawnActorFromClass` "/Game/SHContent/POI/BP_POI_Device_SPJK.BP_POI_Device_SPJK_C" (`KismetMathLibrary.MakeTransform` _enginecoordinates) "AlwaysSpawn" "MultiplyWithRoot" null null))
      (set `local.thePOI` _returnvalue_7))
    (:`7`
      (bind _returnvalue_8 (`|SpawnActorFromClass` "/Game/SHContent/POI/BP_POI_Device_Car.BP_POI_Device_Car_C" (`KismetMathLibrary.MakeTransform` (0.0 0.0 0.0)) "AlwaysSpawn" "MultiplyWithRoot" null null))
      (set `local.thePOI` _returnvalue_8)))
  (return (`local.thePOI`)))

(fn `CreatePOIActor`
  (params (JsonData :type "JsonLibraryObject Structure"))
  (locals (POIJson :type "JsonLibraryObject Structure") (POIActor :type "POIBase Object Reference"))
  (bind _returnvalue (`KismetMathLibrary.MakeTransform` (0.0 0.0 0.0)))
  (bind _poijson (`local.POIJson`))
  (bind _poiactor (`local.POIActor`))
  (bind _poiactor_2 (`local.POIActor`))
  (bind _id (`POIBase.ID` _poiactor_2))
  (if (not (`BlueprintMapLibrary.Map_Contains` (`self.RuntimeMap`) (`JsonLibraryHelpers.JsonObject_GetString` JsonData "ID")))
    (set `local.POIJson` JsonData)
    (switch `int` (`JsonLibraryHelpers.JsonObject_GetInteger` JsonData "StyleType")
      (:`1`
        (bind _returnvalue_2 (`|SpawnActorFromClass` "/Game/SHContent/POI/BP_POI_AreaPeople.BP_POI_AreaPeople_C" _returnvalue "AlwaysSpawn" "MultiplyWithRoot" null null))
        (set `local.POIActor` _returnvalue_2))
      (:`2`
        (bind _returnvalue_3 (`|SpawnActorFromClass` "/Game/SHContent/POI/BP_POI_AreaFund.BP_POI_AreaFund_C" _returnvalue "AlwaysSpawn" "MultiplyWithRoot" null null))
        (set `local.POIActor` _returnvalue_3))
      (:`3`
        (bind _returnvalue_4 (`|SpawnActorFromClass` "/Game/SHContent/POI/BP_POI_AreaPlan.BP_POI_AreaPlan_C" _returnvalue "AlwaysSpawn" "MultiplyWithRoot" null null))
        (set `local.POIActor` _returnvalue_4))
      (:`4`
        (bind _returnvalue_5 (`|SpawnActorFromClass` "/Game/SHContent/POI/BP_POI_AreaBuild.BP_POI_AreaBuild_C" _returnvalue "AlwaysSpawn" "MultiplyWithRoot" null null))
        (set `local.POIActor` _returnvalue_5))
      (:`5`
        (bind _returnvalue_6 (`|SpawnActorFromClass` "/Game/SHContent/POI/BP_POI_AreaOrder.BP_POI_AreaOrder_C" _returnvalue "AlwaysSpawn" "MultiplyWithRoot" null null))
        (set `local.POIActor` _returnvalue_6))
      (:`6`
        (bind _returnvalue_7 (`|SpawnActorFromClass` "/Game/SHContent/POI/BP_POI_AreaEvent.BP_POI_AreaEvent_C" _returnvalue "AlwaysSpawn" "MultiplyWithRoot" null null))
        (set `local.POIActor` _returnvalue_7))
      (:`7`
        (bind _returnvalue_8 (`|SpawnActorFromClass` "/Game/SHContent/POI/BP_POI_Warning.BP_POI_Warning_C" _returnvalue "AlwaysSpawn" "MultiplyWithRoot" null null))
        (set `local.POIActor` _returnvalue_8))
      (:`8`
        (bind _returnvalue_9 (`|SpawnActorFromClass` "/Game/SHContent/POI/BP_POI_WSCLC.BP_POI_WSCLC_C" _returnvalue "AlwaysSpawn" "MultiplyWithRoot" null null))
        (set `local.POIActor` _returnvalue_9))
      (:`9`
        (bind _poiactor_3 (`self.CreateDevice` JsonData))
        (set `local.POIActor` _poiactor_3))
      (:`10`
        (bind _returnvalue_10 (`|SpawnActorFromClass` "/Game/SHContent/POI/BP_POI_PeopleStatus.BP_POI_PeopleStatus_C" _returnvalue "AlwaysSpawn" "MultiplyWithRoot" null null))
        (set `local.POIActor` _returnvalue_10))
      (:`11`
        (bind _returnvalue_11 (`|SpawnActorFromClass` "/Game/SHContent/POI/BP_POI_ProjectFund.BP_POI_ProjectFund_C" _returnvalue "AlwaysSpawn" "MultiplyWithRoot" null null))
        (set `local.POIActor` _returnvalue_11))
      (:`12`
        (bind _returnvalue_12 (`|SpawnActorFromClass` "/Game/SHContent/POI/BP_POI_ProjectPlan.BP_POI_ProjectPlan_C" _returnvalue "AlwaysSpawn" "MultiplyWithRoot" null null))
        (set `local.POIActor` _returnvalue_12))
      (:`13`
        (bind _returnvalue_13 (`|SpawnActorFromClass` "/Game/SHContent/POI/BP_POI_ProjectBuild.BP_POI_ProjectBuild_C" _returnvalue "AlwaysSpawn" "MultiplyWithRoot" null null))
        (set `local.POIActor` _returnvalue_13))
      (:`14`
        (bind _returnvalue_14 (`|SpawnActorFromClass` "/Game/SHContent/POI/BP_POI_Device_PlanPoint.BP_POI_Device_PlanPoint_C" _returnvalue "AlwaysSpawn" "MultiplyWithRoot" null null))
        (set `local.POIActor` _returnvalue_14))
      (:`15`
        (bind _returnvalue_15 (`|SpawnActorFromClass` "/Game/SHContent/POI/BP_POI_Device_ErrorPoint.BP_POI_Device_ErrorPoint_C" _returnvalue "AlwaysSpawn" "MultiplyWithRoot" null null))
        (set `local.POIActor` _returnvalue_15))
      (:`16`
        (bind _returnvalue_16 (`|SpawnActorFromClass` "/Game/SHContent/POI/BP_POI_Device_DiseasePoint.BP_POI_Device_DiseasePoint_C" _returnvalue "AlwaysSpawn" "MultiplyWithRoot" null null))
        (set `local.POIActor` _returnvalue_16))
      (:`17`
        (bind _returnvalue_17 (`|SpawnActorFromClass` "/Game/SHContent/POI/BP_POI_WorkOrder.BP_POI_WorkOrder_C" _returnvalue "AlwaysSpawn" "MultiplyWithRoot" null null))
        (set `local.POIActor` _returnvalue_17)))
    (bind _enginecoordinates (`GeoReferencingSystem.GeographicToEngine` (`GeoReferencingSystem.GetGeoReferencingSystem`) (make `GeographicCoordinates` (`JsonLibraryHelpers.JsonObject_GetFloat` (`local.POIJson`) "X") (`JsonLibraryHelpers.JsonObject_GetFloat` (`local.POIJson`) "Y") (`JsonLibraryHelpers.JsonObject_GetFloat` (`local.POIJson`) "Z"))))
    (`self.K2_SetActorLocation` (`local.POIActor`) _enginecoordinates false false)
    (set `POIBase.ID` (`JsonLibraryHelpers.JsonObject_GetString` _poijson "ID") _poiactor)
    (set `POIBase.Type` (`JsonLibraryHelpers.JsonObject_GetString` (`local.POIJson`) "Type") _poiactor)
    (bind _returnvalue_18 (`JsonLibraryHelpers.JsonObject_GetObject` _poijson "JsonValue"))
    (bind _returnvalue_19 (`JsonLibraryHelpers.JsonObject_Stringify` _returnvalue_18))
    (set `POIBase.JsonValue` _returnvalue_19 _poiactor)
    (`POIBase.UpdateJson` _poiactor)
    (if (`KismetStringLibrary.IsEmpty` _id)
      (`KismetSystemLibrary.PrintString` "创建POI失败")
      (else
        (`BlueprintMapLibrary.Map_Add` (`self.RuntimeMap`) _id _poiactor_2)))))

(fn `CreatePOIByData`
  (params (InPOIData :type "POIData Structure"))
  (locals (POIData :type "POIData Structure") (POIActor :type "POIBase Object Reference") (ThePOI :type "/Game/SHContent/Blueprint/BP_POIBase Object Reference"))
  (bind _thepoi (`local.ThePOI`))
  (bind _output_get (set `local.POIData` InPOIData))
  (bind _returnvalue (`self.GetRuntimeActor` (`.ID` (break `POIData` _output_get))))
  (`/Engine/EditorBlueprintResources/StandardMacros.IsValid` _returnvalue
    (:`Is Valid`
      (`self.SetActorHiddenInGame` _returnvalue false))
    (:`Is Not Valid`
      (bind (_id _displayname _geolocation _styletype _eventtype _jsonobject) (break `POIData` _output_get))
      (bind _enginecoordinates (`GeoReferencingSystem.GeographicToEngine` (`GeoReferencingSystem.GetGeoReferencingSystem`) (make `GeographicCoordinates` (.x _geolocation) (.y _geolocation))))
      (switch `int` (`JsonLibraryHelpers.JsonObject_GetInteger` _jsonobject "deviceType")
        (:`1`
          (bind _returnvalue_2 (`|SpawnActorFromClass` "/Game/SHContent/POI/BP_POI_Device_LLJ.BP_POI_Device_LLJ_C" (`KismetMathLibrary.MakeTransform` _enginecoordinates) "AlwaysSpawn" "MultiplyWithRoot" null null))
          (set `local.ThePOI` _returnvalue_2))
        (:`2`
          (bind _returnvalue_3 (`|SpawnActorFromClass` "/Game/SHContent/POI/BP_POI_Device_YWJ.BP_POI_Device_YWJ_C" (`KismetMathLibrary.MakeTransform` _enginecoordinates) "AlwaysSpawn" "MultiplyWithRoot" null null))
          (set `local.ThePOI` _returnvalue_3))
        (:`3`
          (bind _returnvalue_4 (`|SpawnActorFromClass` "/Game/SHContent/POI/BP_POI_Device_ZNBZ.BP_POI_Device_ZNBZ_C" (`KismetMathLibrary.MakeTransform` _enginecoordinates) "AlwaysSpawn" "MultiplyWithRoot" null null))
          (set `local.ThePOI` _returnvalue_4))
        (:`4`
          (bind _returnvalue_5 (`|SpawnActorFromClass` "/Game/SHContent/POI/BP_POI_Device_SZJCY.BP_POI_Device_SZJCY_C" (`KismetMathLibrary.MakeTransform` _enginecoordinates) "AlwaysSpawn" "MultiplyWithRoot" null null))
          (set `local.ThePOI` _returnvalue_5))
        (:`5`
          (bind _returnvalue_6 (`|SpawnActorFromClass` "/Game/SHContent/POI/BP_POI_Device_QTJC.BP_POI_Device_QTJC_C" (`KismetMathLibrary.MakeTransform` _enginecoordinates) "AlwaysSpawn" "MultiplyWithRoot" null null))
          (set `local.ThePOI` _returnvalue_6))
        (:`6`
          (bind _returnvalue_7 (`|SpawnActorFromClass` "/Game/SHContent/POI/BP_POI_Device_SPJK.BP_POI_Device_SPJK_C" (`KismetMathLibrary.MakeTransform` _enginecoordinates) "AlwaysSpawn" "MultiplyWithRoot" null null))
          (set `local.ThePOI` _returnvalue_7)))
      (`POIBase.UpdateJson` _thepoi)
      (bind (_id_2 _displayname_2 _geolocation_2 _styletype_2 _eventtype_2 _jsonobject_2) (break `POIData` _output_get))
      (set `POIBase.ID` _id_2 _thepoi)
      (bind _returnvalue_8 (`JsonLibraryHelpers.JsonObject_Stringify` _jsonobject_2))
      (set `POIBase.JsonValue` _returnvalue_8 _thepoi)
      (`POIBase.UpdateJson` _thepoi)
      (`BlueprintMapLibrary.Map_Add` (`self.RuntimeMap`) _id_2 _thepoi))))

(fn `CreatePOIByDataList`
  (params (JsonData :type "JsonLibraryObject Structure"))
  (`QuadtreeSceneComponent.ClearAllNode` (`self.QuadtreeScene`))
  (bind _returnvalue (`JsonLibraryHelpers.JsonObject_GetValue` JsonData "DataList"))
  (bind _returnvalue_2 (`JsonLibraryHelpers.ToArray` _returnvalue))
  (for _array_element _returnvalue_2
    (bind _returnvalue_3 (`JsonLibraryHelpers.ToObject` _array_element))
    (bind _returnvalue_4 (`JsonLibraryHelpers.JsonObject_GetObject` _returnvalue_3 "JsonValue"))
    (`QuadtreeSceneComponent.CreateTreeNode` (`self.QuadtreeScene`) (make `POIData` (`JsonLibraryHelpers.JsonObject_GetString` _returnvalue_3 "ID") "" (`KismetMathLibrary.MakeVector` (`JsonLibraryHelpers.JsonObject_GetFloat` _returnvalue_3 "X") (`JsonLibraryHelpers.JsonObject_GetFloat` _returnvalue_3 "Y")) (`JsonLibraryHelpers.JsonObject_GetInteger` _returnvalue_3 "StyleType") (`JsonLibraryHelpers.JsonObject_GetString` _returnvalue_3 "Type") _returnvalue_4)))
  (`QuadtreeSceneComponent.Update` (`self.QuadtreeScene`) 10))

(fn `DeletePOIByData`
  (params (InPOIData :type "POIData Structure"))
  (`self.RemoveRuntimeActor` (`.ID` (break `POIData` InPOIData))))

(fn `OnClickedEvent`
  (params (PickActor :type "Actor Object Reference") (PickComponent :type "PrimitiveComponent Object Reference"))
  (bind _componenttags (`ActorComponent.ComponentTags` (`self.CurrentPickComponent`)))
  (`/Engine/EditorBlueprintResources/StandardMacros.IsValid` (`self.CurrentPickComponent`)
    (:`Is Valid`
      (if (`KismetArrayLibrary.Array_IsEmpty` _componenttags)
        (set `self.CurrentPickComponent` null)
        (`KismetSystemLibrary.PrintString` "点击其他组件")
        (else
          (`PrimitiveComponent.SetMaterial` (`self.CurrentPickComponent`) 0 "/Game/Meshes/ShiGong/VFX_ShiGongCover/M_VFX_ProjectActive.M_VFX_ProjectActive")
          (bind _returnvalue (`self.RigelLevel`))
          (bind _returnvalue_2 (`self.GetRuntimeActor` _returnvalue (`KismetStringLibrary.Concat_StrStr` "Build_" (`KismetStringLibrary.Conv_NameToString` (`|GetArrayItem` _componenttags)))))
          (`/Engine/EditorBlueprintResources/StandardMacros.IsValid` _returnvalue_2
            (:`Is Valid`
              (bind _asbp_poi_project_build (cast `/Game/SHContent/POI/BP_POI_ProjectBuild` _returnvalue_2))
              (`/Game/SHContent/POI/BP_POI_ProjectBuild.SetPOIVisible` _asbp_poi_project_build false)
              (set `self.CurrentPickComponent` null)
              (`KismetSystemLibrary.PrintString` "取消老节点")
              (bind _output_get (set `self.CurrentPickComponent` PickComponent :!label _label))
              (bind _componenttags_2 (`ActorComponent.ComponentTags` _output_get))
              (if (not (`KismetArrayLibrary.Array_IsEmpty` _componenttags_2))
                (`PrimitiveComponent.SetMaterial` (`self.CurrentPickComponent`) 0 "/Game/Meshes/ShiGong/VFX_ShiGongCover/M_VFX_ProjectActive.M_VFX_ProjectActive")
                (bind _output_get_2 (set `self.CurrentPickComponent` PickComponent))
                (`PrimitiveComponent.SetMaterial` _output_get_2 0 "/Game/Meshes/ShiGong/VFX_ShiGongCover/M_VFX_ProjectHightlight.M_VFX_ProjectHightlight")
                (bind _returnvalue_3 (`self.RigelLevel`))
                (bind _returnvalue_4 (`self.GetRuntimeActor` _returnvalue_3 (`KismetStringLibrary.Concat_StrStr` "Build_" (`KismetStringLibrary.Conv_NameToString` (`|GetArrayItem` _componenttags_2)))))
                (`/Engine/EditorBlueprintResources/StandardMacros.IsValid` _returnvalue_4
                  (:`Is Valid`
                    (bind _asbp_poi_project_build_2 (cast `/Game/SHContent/POI/BP_POI_ProjectBuild` _returnvalue_4))
                    (`/Game/SHContent/POI/BP_POI_ProjectBuild.SetPOIVisible` _asbp_poi_project_build_2 true)))))))))
    (:`Is Not Valid`
      (goto _label))))

(fn `PlayerMedia`
  (params (JsonData :type "JsonLibraryObject Structure"))
  (bind _vedioplayer (`self.VedioPlayer`))
  (`/Engine/EditorBlueprintResources/StandardMacros.IsValid` (`self.VedioPlayer`)
    (:`Is Valid`
      _)
    (:`Is Not Valid`
      (bind _returnvalue (`|CreateWidget` "/Rigel/Blueprints/Media/BP_VlcPlayerWidget.BP_VlcPlayerWidget_C"))
      (set `self.VedioPlayer` _returnvalue)))
  (if (not (`Widget.IsInViewport` (`self.VedioPlayer`)))
    (`UserWidget.AddToViewport` (`self.VedioPlayer`) 0)
    (`UserWidget.SetDesiredSizeInViewport` _vedioplayer (1000.0 800.0))
    (`UserWidget.SetPositionInViewport` _vedioplayer (500.0 300.0) true))
  (`/Rigel/Blueprints/Media/BP_VlcPlayerWidget.PlayURL` (`self.VedioPlayer`) JsonData))

(fn `Set Pipe Vector Layer`
  (params (JsonData :type "JsonLibraryObject Structure"))
  (bind _world (`self.World`))
  (`/Engine/EditorBlueprintResources/StandardMacros.IsValid` _world
    (:`Is Valid`
      (bind _ascesium_web_map_service_raster_overlay (cast `CesiumWebMapServiceRasterOverlay` (`|GetArrayItem` (`self.GetComponentsByTag` _world "/Script/Engine.ActorComponent" "VectorPipe"))))
      (set `CesiumWebMapServiceRasterOverlay.Layers` (`JsonLibraryHelpers.JsonObject_GetString` JsonData "Layers") _ascesium_web_map_service_raster_overlay)
      (`CesiumRasterOverlay.Refresh` _ascesium_web_map_service_raster_overlay))))

(fn `SetPeoplePathPoints`
  (params (JsonData :type "JsonLibraryObject Structure"))
  (`KismetArrayLibrary.Array_Clear` (`self.PeoplePointList`))
  (bind _returnvalue (`JsonLibraryHelpers.JsonObject_GetArray` JsonData "Data"))
  (for _array_element _returnvalue
    (bind _returnvalue_2 (`JsonLibraryHelpers.ToObject` _array_element))
    (bind _enginecoordinates (`GeoReferencingSystem.GeographicToEngine` (`GeoReferencingSystem.GetGeoReferencingSystem`) (make `GeographicCoordinates` (`JsonLibraryHelpers.JsonObject_GetFloat` _returnvalue_2 "longitude") (`JsonLibraryHelpers.JsonObject_GetFloat` _returnvalue_2 "latitude") 50.0)))
    (`KismetArrayLibrary.Array_Add` (`self.PeoplePointList`) _enginecoordinates))
  (bind _returnvalue_3 (`self.FindActor` "BP_PeopleTracer"))
  (bind _asbp_people_tracer (cast `/Game/SHContent/Blueprint/BP_PeopleTracer` _returnvalue_3))
  (`/Game/SHContent/Blueprint/BP_PeopleTracer.AddPoints` _asbp_people_tracer (`self.PeoplePointList`)))

(fn `SetServerVisible`
  (params (JsonData :type "JsonLibraryObject Structure"))
  (bind _returnvalue (`self.FindActor` "World"))
  (`/Engine/EditorBlueprintResources/StandardMacros.IsValid` _returnvalue
    (:`Is Valid`
      (bind _returnvalue_2 (`self.GetComponentsByTag` _returnvalue "/Script/Engine.ActorComponent" (`KismetStringLibrary.Conv_StringToName` (`JsonLibraryHelpers.JsonObject_GetString` JsonData "LayerID"))))
      (if (not (`KismetArrayLibrary.Array_IsEmpty` _returnvalue_2))
        (`ActorComponent.SetActive` (`|GetArrayItem` _returnvalue_2) (`JsonLibraryHelpers.JsonObject_GetBoolean` JsonData "Visible") false)))))

(fn `UserConstructionScript`)