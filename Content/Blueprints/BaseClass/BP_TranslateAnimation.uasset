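; BP_TranslateAnimation is a base actor Blueprint that slides itself in a straight line from StartTransform's location toward EndTransform's location.
; PlayAnimation resets the actor to the start and sets duration and visibility, hiding it again if not playing.
; Each externally triggered AnimationEvent applies a fixed offset assuming 30 calls per second; Tick is unused.
; It stops once RunningTime exceeds Duration, though nothing here increments RunningTime.
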(event `self.AnimationEvent`
  (bind _endtransform_location (`KismetMathLibrary.BreakTransform` (`self.EndTransform`)))
  (bind _starttransform_location (`KismetMathLibrary.BreakTransform` (`self.StartTransform`)))
  (if (`self.IsPlaying`)
    (`self.K2_AddActorWorldOffset` (/ (- _endtransform_location _starttransform_location) (* (`self.Duration`) 30.0)))
    (if (> (`self.RunningTime`) (`self.Duration`))
      (set `self.IsPlaying` false)
      (set `self.RunningTime` 0.0))))

(event `self.ResetAnimation`
  (bind _starttransform_location (`KismetMathLibrary.BreakTransform` (`self.StartTransform`)))
  (`self.K2_SetActorLocation` _starttransform_location)
  (`self.SetActorHiddenInGame` true))

(event `self.PlayAnimation`
  (params (isPlaying :type Boolean) (PlayDuration :type "Float (single-precision)"))
  (`self.ResetAnimation`)
  (set `self.IsPlaying` isPlaying)
  (set `self.Duration` PlayDuration)
  (`self.SetActorHiddenInGame` false)
  (if (not isPlaying)
    (`self.ResetAnimation`)))

(fn `UserConstructionScript`)